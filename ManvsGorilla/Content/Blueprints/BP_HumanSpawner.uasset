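; BP_HumanSpawner spawns a wave of BP_Human actors at random navigable points around itself and shows the human count on a HUD.
; BeginPlay creates the WB_Humans widget, which each spawned human receives as a reference.
; SpawnHumans maps the Wave index to a head count, spawns that many within a fixed radius, then writes the total to the widget and adds it to the viewport.
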(event Custom|SpawnHumans
  (params (Wave :type Integer))
  (bind _humanwidgetref (Variables|Default|GetHumanWidgetRef))
  (Variables|Default|SetHumans 0)
  (for _index (range 0 (- (Utilities|Select :Index Wave :Option%200 10 :Option%201 25 :Option%202 50 :Option%203 100) 1))
    (Game|SpawnActorfromClass "/Game/Blueprints/BP_Human.BP_Human_C" (Math|Conversions|ToTransform(Vector) (.RandomLocation (AI|Navigation|GetRandomReachablePointinRadius (Transformation|GetActorLocation) 7e+03 0 0))) "AdjustIfPossibleButAlwaysSpawn" "MultiplyWithRoot" 0 (Variables|Default|GetHumanWidgetRef) 0)
    (Math|Integer|IncrementInt (Variables|Default|GetHumans)))
  (Variables|/Game/Widgets/WB_Humans.WB_Humans_C|SetHumans _humanwidgetref (Variables|Default|GetHumans))
  (UserInterface|Viewport|AddtoViewport _humanwidgetref 0))

(event EventBeginPlay
  (bind _returnvalue (UserInterface|CreateWidget "/Game/Widgets/WB_Humans.WB_Humans_C"))
  (Variables|Default|SetHumanWidgetRef _returnvalue))

(fn ConstructionScript)