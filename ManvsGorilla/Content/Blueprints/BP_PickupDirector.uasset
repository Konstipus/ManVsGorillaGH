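; Director actor that periodically spawns BP_Pickup health pickups at random points inside its Box component's bounds.
; A looping timer started on BeginPlay drives the spawning, and each new pickup is tracked in PickupArray.
; ResetPickups stops the timer and destroys the tracked pickups without emptying the array, while RestartPickupSpawning starts the same timer again.
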(event Custom|SpawnHealthPickup
  (bind _box (Variables|Default|GetBox))
  (bind (_origin _boxextent) (Collision|GetComponentBounds _box))
  (bind _returnvalue (Game|SpawnActorfromClass "/Game/Blueprints/BP_Pickup.BP_Pickup_C" (Math|Conversions|ToTransform(Vector) (Math|Random|RandomPointinBoundingBox _origin _boxextent)) "Undefined" "MultiplyWithRoot" 0 0))
  (Utilities|Array|AddUnique (Variables|Default|GetPickupArray) _returnvalue))

(event Custom|ResetPickups
  (Utilities|Time|ClearandInvalidateTimerbyHandle (stale Custom|RestartPickupSpawning _returnvalue))
  (for _array_element (Variables|Default|GetPickupArray)
    (Actor|DestroyActor _array_element)))

(event Custom|RestartPickupSpawning
  (bind _returnvalue (Utilities|Time|SetTimerbyEvent (delegate Custom|SpawnHealthPickup) 5.0 true)))

(event EventBeginPlay
  (bind _returnvalue (Utilities|Time|SetTimerbyEvent (delegate Custom|SpawnHealthPickup) 5.0 true)))

(fn ConstructionScript)