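; Game mode for a wave-based gorilla game that spawns the player, runs the waves and ends with a game-over screen.
; On BeginPlay it possesses a gorilla at a random PlayerStart, finds the human spawner and pickup director, and starts the first wave.
; Timed widgets announce waves and completions; LevelCompleted resets pickups, then restores health and advances, or ends after the last wave.
; A looping timer tracks elapsed minutes and seconds.
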(event Custom|UpdateTimer
  (bind _returnvalue (Utilities|Time|GetGameTimeinSeconds))
  (bind _returnvalue_2 (Math|Timespan|FromSeconds _returnvalue))
  ;[0.15 0.15 0.15 0.5] Timer
  (Variables|Default|SetSeconds (.seconds _returnvalue_2))
  (Variables|Default|SetMinutes (.minutes _returnvalue_2)))

(event Custom|LevelCompleted
  ;[0.15 0.15 0.15 0.5] On wave beaten
  (Default|ResetPickups (Variables|Default|GetPickupDirectorRef))
  (bind _returnvalue (UserInterface|CreateWidget "/Game/Widgets/WB_LevelCompleted.WB_LevelCompleted_C"))
  (UserInterface|Viewport|AddtoViewport _returnvalue 0)
  (Utilities|FlowControl|Delay 3.0)
  (Widget|RemovefromParent _returnvalue)
  (Widget|RemovefromParent (Variables|/Game/Blueprints/BP_HumanSpawner.BP_HumanSpawner_C|GetHumanWidgetRef (Variables|Default|GetHumanSpawnerRef)))
  (if (>= (Variables|Default|GetWaveNumber) 3)
    (bind _returnvalue_2 (UserInterface|CreateWidget "/Game/Widgets/WB_GameOver.WB_GameOver_C"))
    (UserInterface|Viewport|AddtoViewport _returnvalue_2 0)
    (else
      (bind _result (Math|Integer|IncrementInt (Variables|Default|GetWaveNumber))
        (:%20%20
          (Utilities|FlowControl|Delay 3.0)
          (CallFunction|StartWave _result)
          (Default|RestartPickupSpawning (Variables|Default|GetPickupDirectorRef))
          (Default|ResetHealth (Variables|Default|GetPlayerPawnRef)))))))

(event Custom|StartTimer
  ;[0.15 0.15 0.15 0.5] On wave beaten
  ;;[0.15 0.15 0.15 0.5] Timer
  (Utilities|Time|SetTimerbyEvent (delegate Custom|UpdateTimer) 1.0 true))

(event Custom|StartWave
  (params (WaveNumber :type Integer))
  ;[0.15 0.15 0.15 0.5] StartWave
  (bind _returnvalue (UserInterface|CreateWidget "/Game/Widgets/WB_StartWave.WB_StartWave_C" 0 WaveNumber))
  (UserInterface|Viewport|AddtoViewport _returnvalue 0)
  (Utilities|FlowControl|Delay 3.0)
  (Widget|RemovefromParent _returnvalue)
  (Default|SpawnHumans (Variables|Default|GetHumanSpawnerRef)))

(event Custom|SpawnPlayer
  (bind _returnvalue (Game|GetPlayerController 0))
  ;[0.15 0.15 0.15 0.5] Spawn player
  (bind _outactors (Actor|GetAllActorsOfClass "/Script/Engine.PlayerStart"))
  (bind _returnvalue_2 (Game|SpawnActorfromClass "/Game/Blueprints/BP_Gorilla.BP_Gorilla_C" (Transformation|GetActorTransform (.OutItem (Utilities|Array|Random _outactors))) "Undefined" "MultiplyWithRoot" 0 0))
  (bind _output_get (Variables|Default|SetPlayerPawnRef _returnvalue_2))
  (Pawn|Possess _returnvalue _output_get)
  (Input|EnableInput _output_get _returnvalue))

(event EventBeginPlay
  (CallFunction|SpawnPlayer)
  (CallFunction|StartTimer)
  (bind _returnvalue (Actor|GetActorOfClass "/Game/Blueprints/BP_HumanSpawner.BP_HumanSpawner_C"))
  (Variables|Default|SetHumanSpawnerRef _returnvalue)
  (bind _returnvalue_2 (Actor|GetActorOfClass "/Game/Blueprints/BP_PickupDirector.BP_PickupDirector_C"))
  (Variables|Default|SetPickupDirectorRef _returnvalue_2)
  (CallFunction|StartWave))

(fn ConstructionScript)