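; Player-controlled gorilla character with camera-relative Enhanced Input movement, a montage melee attack, health and death.
; GorillaArm overlaps apply damage to other actors, with arm collision off by default and switched through ToggleGorillaCollision.
; Damage and ResetHealth update the health HUD created beside a timer widget at BeginPlay; death disables input, plays a montage, snarls and destroys the actor.
; ShakeScreen adds camera shake and snarl; look input is unwired.
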(event OnComponentBeginOverlap(GorillaArm)
  (params (OverlappedComponent :type Primitive%20Component%20Object%20Reference) (OtherActor :type Actor%20Object%20Reference) (OtherComp :type Primitive%20Component%20Object%20Reference) (OtherBodyIndex :type Integer) (bFromSweep :type Boolean) (SweepResult :type Hit%20Result%20Structure%20%28by%20ref%29))
  ;[0.15 0.15 0.15 0.5] ApplyDmgonAttack
  (if (not (== OtherActor self))
    (Game|Damage|ApplyDamage OtherActor 1.0 0 self)))

(event Custom|ToggleGorillaCollision
  (params (True? :type Boolean))
  (bind _gorillaarm (Variables|Default|GetGorillaArm))
  ;[0.15 0.15 0.15 0.5] ToggleHandColl
  (if True?
    (Collision|SetCollisionEnabled _gorillaarm "QueryAndPhysics")
    (else
      (Collision|SetCollisionEnabled _gorillaarm "NoCollision"))))

(event Custom|ShakeScreen
  (Camera|PlayWorldCameraShake "/Game/Blueprints/BP_CameraShake.BP_CameraShake_C" (Transformation|GetActorLocation) 0.0 1e+03)
  (Audio|PlaySoundatLocation "/Game/SFX/Gorillagrunts/SC_GorillaSnarl.SC_GorillaSnarl" (Transformation|GetActorLocation) "0, 0, 0" 1.0 1.0 0.0 0 0 0 0))

(event Custom|ResetHealth
  (Variables|Default|SetHealth (Variables|Default|GetMaxHealth))
  (Default|UpdateHealthBar (Variables|Default|GetGorillaHud)))

(event Input|EnhancedActionEvents|EnhancedInputActionIA_Move
  (params (ActionValue :type Vector%202D%20Structure) (ElapsedSeconds :type Float%20%28double-precision%29) (TriggeredSeconds :type Float%20%28double-precision%29) (InputAction :type Input%20Action%20Object%20Reference :default "/Game/Input/IA_Move.IA_Move"))
  (bind _returnvalue (Pawn|GetControlRotation :!class /Script/Engine.Pawn))
  ;[0.15 0.15 0.15 0.5] Movement
  ;;[0.15 0.15 0.15 0.5] L/R
  (Pawn|Input|AddMovementInput (Math|Vector|GetRightVector (Math|Rotator|MakeRotator (.roll _returnvalue) 0.0 (.yaw _returnvalue))) (.x ActionValue) false)
  ;;[0.15 0.15 0.15 0.5] F/B
  (Pawn|Input|AddMovementInput (Math|Vector|GetForwardVector (Math|Rotator|MakeRotator 0.0 0.0 (.yaw (Pawn|GetControlRotation :!class /Script/Engine.Pawn)))) (.y ActionValue) false))

(event Input|EnhancedActionEvents|EnhancedInputActionIA_Look
  (params (ActionValue :type Vector%202D%20Structure) (ElapsedSeconds :type Float%20%28double-precision%29) (TriggeredSeconds :type Float%20%28double-precision%29) (InputAction :type Input%20Action%20Object%20Reference :default "/Game/Input/IA_Look.IA_Look")))

(event Input|EnhancedActionEvents|EnhancedInputActionIA_Attack
  (params (ActionValue :type Boolean) (ElapsedSeconds :type Float%20%28double-precision%29) (TriggeredSeconds :type Float%20%28double-precision%29) (InputAction :type Input%20Action%20Object%20Reference :default "/Game/Input/IA_Attack.IA_Attack"))
  ;[0.15 0.15 0.15 0.5] AttackAnimation
  (:Started
    (Utilities|FlowControl|DoOnce false :!label _label
      (:Completed
        (Animation|Montage|PlayMontage (Variables|Character|GetMesh) "/Game/Gorilla/Animations/A_Gorillattackelftarm_Montage.A_Gorillattackelftarm_Montage" 1.7
          (:OnCompleted
            (goto _label Reset))
          (:OnInterrupted
            (goto _label Reset)))))))

(event EventPossessed
  (params (NewController :type Controller%20Object%20Reference))
  ;[0.15 0.15 0.15 0.5] Add Control to the character
  (bind _asplayer_controller (Utilities|Casting|CastToPlayerController NewController))
  (Input|AddMappingContext (PlayerController|LocalPlayerSubsystems|GetEnhancedInputLocalPlayerSubsystem _asplayer_controller) "/Game/Input/IMC_Gorilla.IMC_Gorilla" 0 "(bIgnoreAllPressedKeysUntilRelease=True,bForceImmediately=False,bNotifyUserSettings=False)"))

(event EventBeginPlay
  (Utilities|FlowControl|Sequence
    (:then_0
      (bind _returnvalue (UserInterface|CreateWidget "/Game/Widgets/WB_GorillaHealth.WB_GorillaHealth_C" 0 self))
      (bind _output_get (Variables|Default|SetGorillaHud _returnvalue))
      (UserInterface|Viewport|AddtoViewport _output_get 0)
      (Collision|SetCollisionEnabled (Variables|Default|GetGorillaArm) "NoCollision"))
    (:then_1
      (bind _returnvalue_2 (UserInterface|CreateWidget "/Game/Widgets/WB_Timer.WB_Timer_C"))
      (bind _output_get_2 (Variables|Default|SetTimerRef _returnvalue_2))
      (UserInterface|Viewport|AddtoViewport _output_get_2 0))))

(event Game|Damage|EventAnyDamage
  (params (Damage :type Float%20%28single-precision%29) (DamageType :type Damage%20Type%20Object%20Reference) (InstigatedBy :type Controller%20Object%20Reference) (DamageCauser :type Actor%20Object%20Reference))
  ;[0.15 0.15 0.15 0.5] HandleGorillaReceivingDmg
  (bind _output_get (Variables|Default|SetHealth (- (Variables|Default|GetHealth) Damage)))
  (Default|UpdateHealthBar (Variables|Default|GetGorillaHud))
  (if (<= _output_get 0.0)
    (Utilities|FlowControl|DoOnce false
      (:Completed
        (Input|DisableInput (Game|GetPlayerController 0))
        (Animation|Montage|PlayMontage (Variables|Character|GetMesh) "/Game/Gorilla/Animations/A_gorriladie_Montage.A_gorriladie_Montage"
          (:OnCompleted
            (Audio|PlaySoundatLocation "/Game/SFX/Gorillagrunts/SC_GorillaSnarl.SC_GorillaSnarl" (Transformation|GetActorLocation) "0, 0, 0" 1.0 1.0 0.0 0 0 0 0)
            (Actor|DestroyActor)))))))

(fn ConstructionScript)