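; BP_Pickup is a health pickup actor that heals BP_Gorilla when it overlaps the static mesh.
; A RotatingMovement component spins the mesh, while the Levitate timeline moves the actor vertically by adding its ZPos value to the current location on each update.
; On overlap it adds HealingAmount to the gorilla's health, clamped to MaxHealth, refreshes the HUD health bar and destroys itself.
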(event OnComponentBeginOverlap(StaticMesh)
  (params (OverlappedComponent :type Primitive%20Component%20Object%20Reference) (OtherActor :type Actor%20Object%20Reference) (OtherComp :type Primitive%20Component%20Object%20Reference) (OtherBodyIndex :type Integer) (bFromSweep :type Boolean) (SweepResult :type Hit%20Result%20Structure%20%28by%20ref%29))
  (bind _asbp_gorilla (Utilities|Casting|CastToBP_Gorilla OtherActor))
  (Variables|/Game/Blueprints/BP_Gorilla.BP_Gorilla_C|SetHealth _asbp_gorilla (Math|Float|Clamp(Float) (+ (Variables|/Game/Blueprints/BP_Gorilla.BP_Gorilla_C|GetHealth _asbp_gorilla) (Variables|Default|GetHealingAmount)) 0.0 (Variables|/Game/Blueprints/BP_Gorilla.BP_Gorilla_C|GetMaxHealth _asbp_gorilla)))
  (Default|UpdateHealthBar (Variables|/Game/Blueprints/BP_Gorilla.BP_Gorilla_C|GetGorillaHud _asbp_gorilla))
  (Actor|DestroyActor))

(event EventBeginPlay
  (bind _returnvalue (Transformation|GetActorLocation))
  (Components|Movement|SetUpdatedComponent (Variables|Default|GetRotatingMovement) (Variables|Default|GetStaticMesh))
  (bind _zpos (Timeline|Levitate Play)
    (:Update
      (Transformation|SetActorLocation (Math|Vector|MakeVector (.x _returnvalue) (.y _returnvalue) (+ (.z _returnvalue) _zpos)) false true))))

(fn ConstructionScript)